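; Robot that turns player text into movement or a reply by querying ChatGPT through MyHTTPClient.
; BeginPlay builds an indexed name list of "Target"-tagged actors, which MoveToLocation sends with the player's text.
; After a fixed three-second delay, a negative number moves it to the player, other numbers index a target, and non-numeric text goes to the first-person character's SendToWB.
; The API key is hardcoded; the save-loaded key is unwired.
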(event Custom|MoveToLocation
  (params (Text :type Text))
  (bind _self self)
  (bind _returnvalue (Game|ConstructObjectfromClass "/Script/GPTGame.MyHTTPClient"))
  (Class|MyHTTPClient|SetAPIKey _returnvalue "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")
  (Class|MyHTTPClient|SendChatGPTRequest _returnvalue (Utilities|Text|ToText(String) (Utilities|String|Append "This is Objects list[" (Variables|Default|GetList) "] This is player's input[" (Utilities|String|ToString(Text) Text) "]")))
  (Utilities|FlowControl|Delay 3.0)
  (if (Class|KismetStringLibrary|IsNumeric (Utilities|String|ToString(Text) (Class|MyHTTPClient|GetResponse _returnvalue)))
    (if (< (Math|Conversions|ToInteger(Byte) (Utilities|String|ToString(Text) (Class|MyHTTPClient|GetResponse _returnvalue))) 0)
      (AI|AIMoveTo _self "0, 0, 0" (Game|GetPlayerCharacter 0) 0.0 false
        (:then
          (Development|PrintText (Class|MyHTTPClient|GetResponse _returnvalue) true true "(R=0.000000,G=0.660000,B=1.000000,A=1.000000)" 1003.0 :!label _label))
        (:OnFail
          (Development|PrintString "Hello" :!label _label_2)))
      (elif (Utilities|Array|IsValidIndex (stale EventBeginPlay _output_get))
        (AI|AIMoveTo _self (Transformation|GetActorLocation (Utilities|Array|Get(acopy) (stale EventBeginPlay _output_get) (Math|Conversions|ToInteger(Byte) (Utilities|String|ToString(Text) (Class|MyHTTPClient|GetResponse _returnvalue))))) 0 0.0 false
          (:then
            (goto _label))
          (:OnFail
            (goto _label_2)))))
    (else
      (Development|PrintText (Class|MyHTTPClient|GetResponse _returnvalue) true true "(R=0.000000,G=0.660000,B=1.000000,A=1.000000)" 3.0)
      (bind _outactors (Actor|GetAllActorsOfClass "/Game/FirstPerson/Blueprints/BP_FirstPersonCharacter.BP_FirstPersonCharacter_C"))
      (Default|SendtoWB (Utilities|Array|Get(acopy) _outactors) (Class|MyHTTPClient|GetResponse _returnvalue)))))

(event EventBeginPlay
  (bind _outactors (Actor|GetAllActorswithTag "Target"))
  (bind _output_get (Variables|Default|SetTargetObjects _outactors))
  (for (_array_element _array_index) _output_get
    (Variables|Default|SetList (Utilities|String|Append (Variables|Default|GetList) (Utilities|String|ToString(Integer) _array_index) ": " (Utilities|GetDisplayName _array_element) "; ")))
  (Development|PrintString (Variables|Default|GetList) true true "(R=0.000000,G=0.660000,B=1.000000,A=1.000000)" 1e+02)
  (bind _returnvalue (SaveGame|LoadGamefromSlot "MySlot"))
  (bind _assave_api (Utilities|Casting|CastToSaveAPI _returnvalue)))

(fn ConstructionScript)