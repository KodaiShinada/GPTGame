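; BP_MoveFloor is a second-stage floor actor that moves once enough pressure switches are active.
; SwitchActivated and SwitchDeactivated adjust a count of active switches and compare it to the required number.
; Meeting the threshold plays the FloorActication timeline, otherwise it reverses, driving the Floor's relative Z location from the FloorPosition track.
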(event Custom|SwitchActivated
  (Math|Integer|IncrementInt (Variables|Default|GetPressureSwitchesActive)
    (:%20%20
      (if (>= (Variables|Default|GetPressureSwitchesActive) (Variables|Default|GetPressureSwitchesNeeded))
        (bind _floorposition (Timeline|FloorActication Play)
          (:Update
            (Transformation|SetRelativeLocation (Variables|Default|GetFloor) (Math|Vector|MakeVector 0.0 0.0 _floorposition) false false)))
        (else
          (Timeline|FloorActication Reverse))))))

(event Custom|SwitchDeactivated
  (Math|Integer|DecrementInt (Variables|Default|GetPressureSwitchesActive)
    (:%20%20
      (if (>= (Variables|Default|GetPressureSwitchesActive) (Variables|Default|GetPressureSwitchesNeeded))
        (bind _floorposition (Timeline|FloorActication Play)
          (:Update
            (Transformation|SetRelativeLocation (Variables|Default|GetFloor) (Math|Vector|MakeVector 0.0 0.0 _floorposition) false false)))
        (else
          (Timeline|FloorActication Reverse))))))

(event EventBeginPlay)

(event Collision|EventActorBeginOverlap
  (params (OtherActor :type Actor%20Object%20Reference)))

(event EventTick
  (params (DeltaSeconds :type Float%20%28single-precision%29)))

(fn ConstructionScript)